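; BP_DamageTrigger_Master is a damage volume that repeatedly hurts the FirstPersonCharacter while it overlaps the Trigger component.
; Begin overlap stores the character and starts a looping timer that applies DamageDealt every DamageInterval, so the first hit lands one interval after entry.
; End overlap pauses the timer by handle instead of clearing it, and each new entry sets it again.
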(event OnComponentBeginOverlap(trigger)
  (params (OverlappedComponent :type Primitive%20Component%20Object%20Reference) (OtherActor :type Actor%20Object%20Reference) (OtherComp :type Primitive%20Component%20Object%20Reference) (OtherBodyIndex :type Integer) (bFromSweep :type Boolean) (SweepResult :type Hit%20Result%20Structure%20%28by%20ref%29))
  (bind _asfirst_person_character (Utilities|Casting|CastToFirstPersonCharacter OtherActor))
  (bind _returnvalue (Utilities|Time|SetTimerbyEvent (delegate Custom|OnPlyerInTrigger) (Variables|Default|GetDamage%20Interval) true))
  (Variables|Default|SetTimer%20Damage _returnvalue))

(event OnComponentEndOverlap(trigger)
  (params (OverlappedComponent :type Primitive%20Component%20Object%20Reference) (OtherActor :type Actor%20Object%20Reference) (OtherComp :type Primitive%20Component%20Object%20Reference) (OtherBodyIndex :type Integer))
  (Utilities|Casting|CastToFirstPersonCharacter OtherActor)
  (Utilities|Time|PauseTimerbyHandle (Variables|Default|GetTimer%20Damage)))

(event Custom|OnPlyerInTrigger
  (Game|Damage|ApplyDamage (stale OnComponentBeginOverlap(trigger) _asfirst_person_character) (Variables|Default|GetDamage%20Dealt) 0 0))

(fn ConstructionScript)