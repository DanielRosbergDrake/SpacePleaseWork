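; ElevatorDoorKeycard is an elevator door that opens with the E key when the player holds a keycard.
; Entering its box enables input; pressing E plays a low-pitched sound, then checks HasKeycard on BP_GameInstance.
; A timeline slides the door between start and end positions, feeding its track into VInterpTo as DeltaTime.
; Leaving the box reverses the timeline but never disables input.
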(event OnComponentBeginOverlap(Box)
  (params (OverlappedComponent :type Primitive%20Component%20Object%20Reference) (OtherActor :type Actor%20Object%20Reference) (OtherComp :type Primitive%20Component%20Object%20Reference) (OtherBodyIndex :type Integer) (bFromSweep :type Boolean) (SweepResult :type Hit%20Result%20Structure%20%28by%20ref%29))
  (Input|EnableInput (Game|GetPlayerController 0)))

(event OnComponentEndOverlap(Box)
  (params (OverlappedComponent :type Primitive%20Component%20Object%20Reference) (OtherActor :type Actor%20Object%20Reference) (OtherComp :type Primitive%20Component%20Object%20Reference) (OtherBodyIndex :type Integer))
  (bind _newtrack_0 (Timeline|Timeline_0 Reverse)
    (:Update
      (Transformation|SetRelativeLocation (Variables|Default|GetSPW_ElevatorDoor) (Math|Interpolation|VInterpTo (Variables|Default|GetStartPos) (Variables|Default|GetEndPos) _newtrack_0 0.8) false false))))

(event Input|KeyboardEvents|E
  (params (Key :type Key%20Structure))
  (:Pressed
    (Audio|SpawnSoundatLocation "/Game/FirstPerson/Audio/FirstPersonTemplateWeaponFire02.FirstPersonTemplateWeaponFire02" (Transformation|GetActorLocation) "0, 0, 0" 1e+01 0.005 1.0 0 0)
    (bind _asbp_game_instance (Utilities|Casting|CastToBP_GameInstance (Game|GetGameInstance)))
    (if (Variables|/Game/Root/DRD/Blueprints/BP_GameInstance.BP_GameInstance_C|GetHasKeycard _asbp_game_instance)
      (bind _newtrack_0 (Timeline|Timeline_0 Play)
        (:Update
          (Transformation|SetRelativeLocation (Variables|Default|GetSPW_ElevatorDoor) (Math|Interpolation|VInterpTo (Variables|Default|GetStartPos) (Variables|Default|GetEndPos) _newtrack_0 0.8) false false))))))

(fn ConstructionScript)