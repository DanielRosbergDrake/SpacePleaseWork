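; SPW_EggDestroy is a destructible actor, named as an egg, that can be shot apart and hurts the player on contact.
; Each FirstPersonProjectile hit on its capsule lowers Health, and once that falls to a low threshold the actor spawns a sparks emitter and destroys itself.
; A hit from a FirstPersonCharacter instead applies a small amount of damage to that character.
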(event OnComponentHit(Capsule)
  (params (HitComponent :type Primitive%20Component%20Object%20Reference) (OtherActor :type Actor%20Object%20Reference) (OtherComp :type Primitive%20Component%20Object%20Reference) (NormalImpulse :type Vector :default "0, 0, 0") (Hit :type Hit%20Result%20Structure%20%28by%20ref%29))
  (Utilities|Casting|CastToFirstPersonProjectile OtherActor
    (:then
      (Variables|Default|SetHealth (- (Variables|Default|GetHealth) 1e+01))
      (if (<= (Variables|Default|GetHealth) 5.0)
        (Effects|SpawnEmitteratLocation "/Game/Root/StarterContent/Particles/P_Sparks.P_Sparks" (Transformation|GetActorLocation) "0, 0, 0" "1.500000,1.500000,0.500000")
        (Actor|DestroyActor)))
    (:CastFailed
      (bind _asfirst_person_character (Utilities|Casting|CastToFirstPersonCharacter OtherActor))
      (Game|Damage|ApplyDamage _asfirst_person_character 1.0 0 0))))

(fn ConstructionScript)