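; Door actor that slides two parts, SPWDoorV and SPWDoorH, open or closed when E is pressed.
; Box overlap enables input for player 0, with no matching disable.
; Two E handlers, one also playing a pitched-down weapon-fire sound, play or reverse separate timelines whose track drives VInterpTo DeltaTime between stored positions.
; Tick derives ClosedDoor from Timeline_1 alone, as its branch is hardwired false.
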(event OnComponentBeginOverlap(Box)
  (params (OverlappedComponent :type Primitive%20Component%20Object%20Reference) (OtherActor :type Actor%20Object%20Reference) (OtherComp :type Primitive%20Component%20Object%20Reference) (OtherBodyIndex :type Integer) (bFromSweep :type Boolean) (SweepResult :type Hit%20Result%20Structure%20%28by%20ref%29))
  (Input|EnableInput (Game|GetPlayerController 0)))

(event EventTick
  (params (DeltaSeconds :type Float%20%28single-precision%29))
  (if false
    (Variables|Default|SetClosedDoor (< (stale Input|KeyboardEvents|E _newtrack_0) 1.1))
    (else
      (Variables|Default|SetClosedDoor (< (stale Input|KeyboardEvents|E _newtrack_0) 1.1)))))

(event Input|KeyboardEvents|E
  (params (Key :type Key%20Structure))
  (:Pressed
    (if (Variables|Default|GetClosedDoor)
      (bind _newtrack_0 (Timeline|Timeline_1 Play)
        (:Update
          (Transformation|SetRelativeLocation (Variables|Default|GetSPW_DoorH) (Math|Interpolation|VInterpTo (Variables|Default|GetStartPosH) (Variables|Default|GetEndPosH) _newtrack_0 0.8) false false)))
      (else
        (Timeline|Timeline_1 Reverse)))))

(event Input|KeyboardEvents|E
  (params (Key :type Key%20Structure))
  (:Pressed
    (Audio|SpawnSoundatLocation "/Game/FirstPerson/Audio/FirstPersonTemplateWeaponFire02.FirstPersonTemplateWeaponFire02" (Transformation|GetActorLocation) "0, 0, 0" 1e+01 0.005 1.0 0 0)
    (if (Variables|Default|GetClosedDoor)
      (bind _newtrack_0 (Timeline|Timeline_0 Play)
        (:Update
          (Transformation|SetRelativeLocation (Variables|Default|GetSPW_DoorV) (Math|Interpolation|VInterpTo (Variables|Default|GetStartPosV) (Variables|Default|GetEndPosV) _newtrack_0 0.8) false false)))
      (else
        (Timeline|Timeline_0 Reverse)))))

(fn ConstructionScript)