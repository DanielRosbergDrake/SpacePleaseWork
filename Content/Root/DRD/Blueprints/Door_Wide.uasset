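; Wide double door that slides open when a Pawn enters its Box trigger.
; The overlap plays a timeline that moves the left and right panels between stored start and end relative positions.
; Each update calls VInterpTo from the fixed start, feeding the timeline track in as DeltaTime so it acts as a scaled blend factor.
; The graph has no end-overlap or reverse logic to close the door.
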(event OnComponentBeginOverlap(Box)
  (params (OverlappedComponent :type Primitive%20Component%20Object%20Reference) (OtherActor :type Actor%20Object%20Reference) (OtherComp :type Primitive%20Component%20Object%20Reference) (OtherBodyIndex :type Integer) (bFromSweep :type Boolean) (SweepResult :type Hit%20Result%20Structure%20%28by%20ref%29))
  (Utilities|Casting|CastToPawn OtherActor)
  (bind _newtrack_0 (Timeline|Timeline_0 Play)
    (:Update
      (Transformation|SetRelativeLocation (Variables|Default|GetSPW_Door_Wideleft) (Math|Interpolation|VInterpTo (Variables|Default|GetStartPosLeft) (Variables|Default|GetEndPosLeft) _newtrack_0 0.5) false false)
      (Transformation|SetRelativeLocation (Variables|Default|GetSPW_Door_Wideright) (Math|Interpolation|VInterpTo (Variables|Default|GetStartPosRight) (Variables|Default|GetEndPosRight) _newtrack_0 0.5) false false))))

(fn ConstructionScript)